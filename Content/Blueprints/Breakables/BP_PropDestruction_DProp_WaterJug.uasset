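; Breakable water jug prop that shatters through Chaos destruction and drops a random gem.
; On BeginPlay it fills a treasure list with emerald, sapphire and ruby classes.
; Each GeometryCollection break event plays a pot-break sound at the break location.
; A one-shot flag ensures only the first break spawns a randomly chosen treasure, slightly above the jug's origin.
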(event OnChaosBreakEvent(GeometryCollection)
  (params (BreakEvent :type Chaos%20Break%20Event%20Structure%20%28by%20ref%29))
  (bind _returnvalue (Transformation|GetActorTransform))
  (Audio|PlaySoundatLocation "/Game/Audio/MetaSounds/SFX_PotBreak.SFX_PotBreak" (.location BreakEvent) "0, 0, 0" 1.0 1.0 0.0 0 0 0 0)
  (if (not (Variables|Default|GethasTreasureBeenSpawned))
    (Variables|Default|SethasTreasureBeenSpawned true)
    (Game|SpawnActorfromClass (.OutItem (Utilities|Array|Random (Variables|Default|GetArrayOfTreasures))) (Math|Transform|MakeTransform (Math|Vector|MakeVector (.x (.location _returnvalue)) (.y (.location _returnvalue)) (+ (.z (.location _returnvalue)) 25.0)) (.rotation _returnvalue) (.scale _returnvalue)) "AlwaysSpawn" "MultiplyWithRoot" 0 0)))

(event EventBeginPlay
  (|CallParentFunction)
  (Variables|Default|SethasTreasureBeenSpawned false)
  (Utilities|Array|AddUnique (Variables|Default|GetArrayOfTreasures) "/Game/Blueprints/Items/Pickups/BP_Emerald.BP_Emerald_C")
  (Utilities|Array|AddUnique (Variables|Default|GetArrayOfTreasures) "/Game/Blueprints/Items/Pickups/BP_Sapphire.BP_Sapphire_C")
  (Utilities|Array|AddUnique (Variables|Default|GetArrayOfTreasures) "/Game/Blueprints/Items/Pickups/BP_Ruby.BP_Ruby_C"))

(fn ConstructionScript
  (|CallParentFunction))
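; Destructible metal-stand brazier prop with a flickering fire light, extending a parent prop's break behavior.
; A random-interval timer picks offsets that Tick interpolates the point light toward, while the construction script randomizes its light-function material offset.
; On initial break it spawns a hot-coal Niagara burst facing away from the hit, removes the coals and fire, and plays a timeline that dims and destroys the light.
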(event Custom|LightFlicker01
  (Utilities|IsValid (Variables|Default|GetPointLightPrimary)
    (:Is%20Valid
      (Variables|Default|SetNewLightLocationPrimary (* (Math|Random|RandomUnitVector) (Variables|Default|GetLightFlickerRange)))
      (Utilities|Time|SetTimerbyEvent (delegate Custom|LightFlicker01) (Math|Random|RandomFloatinRange 0.05 0.2)))))

(event EventBeginPlay
  (|CallParentFunction)
  (Variables|Default|SetDefaultLightLocation (Variables|/Script/Engine.SceneComponent|GetRelativeLocation (Variables|Default|GetCoalSpawnLocation)))
  (Variables|Default|SetNewLightLocationPrimary (Variables|Default|GetDefaultLightLocation))
  (Utilities|Time|SetTimerbyEvent (delegate Custom|LightFlicker01) (Math|Random|RandomFloatinRange 0.1 0.5)))

(event EventTick
  (params (DeltaSeconds :type Float%20%28single-precision%29))
  (|CallParentFunction DeltaSeconds)
  (Utilities|IsValid (Variables|Default|GetPointLightPrimary)
    (:Is%20Valid
      (Transformation|SetRelativeLocation (Variables|Default|GetPointLightPrimary) (Math|Interpolation|VInterpTo (Variables|/Script/Engine.SceneComponent|GetRelativeLocation (Variables|Default|GetPointLightPrimary)) (Variables|Default|GetNewLightLocationPrimary) (Utilities|Time|GetWorldDeltaSeconds) 5.0) false false))))

(fn ConstructionScript
  (bind _pointlightprimary (Variables|Default|GetPointLightPrimary))
  (|CallParentFunction)
  (bind _returnvalue (Rendering|Material|CreateDynamicMaterialInstance (Variables|/Script/Engine.LightComponent|GetLightFunctionMaterial _pointlightprimary) "None" "None" :!class /Script/Engine.KismetMaterialLibrary))
  (Rendering|Material|SetScalarParameterValue _returnvalue "RandOffset" (Math|Random|RandomFloatinRange 0.0 1.0) :!class /Script/Engine.MaterialInstanceDynamic)
  (Rendering|Components|Light|SetLightFunctionMaterial _pointlightprimary _returnvalue))

(fn OnInitialBreakChildEvent
  (params (BreakEvent :type Chaos%20Break%20Event%20Structure))
  (bind _coalspawnlocation (Variables|Default|GetCoalSpawnLocation))
  (bind _returnvalue (Transformation|GetWorldLocation _coalspawnlocation))
  (|CallParentFunction BreakEvent)
  (Niagara|SpawnSystematLocation "/Game/PropDestructionSystem/DestructablePropsSamples/SampleProps_Effects/Coals/NS_PropDestruction_Break_HotCoals.NS_PropDestruction_Break_HotCoals" _returnvalue (Math|Rotator|FindLookatRotation (.Location (Utilities|Struct|BreakChaosBreakEvent BreakEvent)) _returnvalue))
  (Utilities|FlowControl|Sequence
    (:then_0
      (bind _brazier_coals (Variables|Default|GetBrazier_Coals)
        (:then
          (Components|DestroyComponent _brazier_coals))
        (:else)))
    (:then_1
      (bind _fireparticlesystem (Variables|Default|GetFireParticleSystem)
        (:then
          (Components|DestroyComponent _fireparticlesystem))
        (:else)))
    (:then_2
      (bind _killlight (Variables|Default|GetKillLight)
        (:then
          (Components|Timeline|PlayfromStart _killlight))
        (:else)))))
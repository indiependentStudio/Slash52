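; Actor component that lets its owner break destructible props by spawning prop destruction field actors.
; On BeginPlay it caches the owner's mesh and capsule via an interface, optionally ensures a weapon trace component, and can attach a push field whose impact velocity follows owner speed each tick.
; Functions spawn bone-attached, standard or swing-directed fields, the latter limited to the hit prop's overlapping anchors, and set capsule response to destructibles.
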(event EventBeginPlay
  (Utilities|FlowControl|Sequence
    (:then_0
      ;[1 0.5391 0] Initially set refs to owning actor's capsule and skeletal mesh components
      (Initilization|SetOwnerRefs)
      (if (Variables|WeaponDestruction|GetbDoWeaponTrace)
        ;[0 1 0.1328] Add trace component to owner
        (CallFunction|AddNeededComponentstoOwner)))
    (:then_1
      ;[0 0.9062 1] Spawn push field if enabled
      (CallFunction|SpawnPushField (Variables|PushForce|GetbUsePushForce)))))

(event EventTick
  (params (DeltaSeconds :type Float%20%28single-precision%29))
  ;[0 1 0.5547] Update push field if enabled
  (CallFunction|UpdatePushForce (Variables|PushForce|GetbUsePushForce)))

(fn SetOwnerRefs
  ;[1 1 1] Set references to the owning actor's skeletal mesh and capsule collision components
  (bind (_weaponmeshcomponent _skeletalmeshcomponent _capsulecomponent) (Class|BPIPropDestructionSource|BPIGetRelevantComponents(Message) (Components|GetOwner)))
  (Utilities|FlowControl|Sequence
    (:then_0
      (Utilities|IsValid _skeletalmeshcomponent
        (:Is%20Valid
          (Variables|Default|SetOwnerSkeletalMeshRef _skeletalmeshcomponent))))
    (:then_1
      (Utilities|IsValid _capsulecomponent
        (:Is%20Valid
          (Variables|Default|SetCapsule%20Component _capsulecomponent))))))

(fn SpawnAttachedDestructionSphere
  (params (F_PropDestructionField_NotifyData :type F%20Prop%20Destruction%20SK%20Field%20Notify%20Data%20Structure%20%28by%20ref%29))
  (bind (_bonename _radius) (Utilities|Struct|BreakF_PropDestruction_SKField_NotifyData F_PropDestructionField_NotifyData))
  (bind _ownerskeletalmeshref (Variables|Default|GetOwnerSkeletalMeshRef)
    (:then
      ;[1 0 0.6562] Spawn a prop destruction field based in input DestructionFieldNotifyData
      (bind _returnvalue (Game|SpawnActorfromClass :Class "/Game/PropDestructionSystem/DestructablePropsCore/BP_PropDestruction_PropDestructionField.BP_PropDestruction_PropDestructionField_C" :SpawnTransform (Transformation|GetSocketTransform _ownerskeletalmeshref _bonename "RTS_World") :CollisionHandlingOverride "Undefined" :SphereRadius _radius :bDebug (Utilities|Select :Index (Variables|Debug|GetDebugLevel) :NewEnumerator0 false :NewEnumerator1 true :NewEnumerator2 true) :Instigator 0))
      ;;[0.8516 0 1] Attach spawned field to owning actor's skeletal mesh based on bone name in DesructionFieldNotifyData
      (Transformation|AttachComponentToComponent _returnvalue (Variables|Default|GetOwnerSkeletalMeshRef) _bonename "SnapToTarget" "SnapToTarget" "SnapToTarget" true)
      (return true _returnvalue))
    (:else)))

(fn SetCapsuleCollisionResponsetoDestructable
  (params (NewResponse :type ECollisionResponse%20Enum :default "ECR_Ignore"))
  ;[0 1 0.8359] Change the collision response of the owning actor's capsule component to destructables
  (bind _capsule_component (Variables|Default|GetCapsule%20Component)
    (:then
      (Collision|SetCollisionResponsetoChannel _capsule_component "ECC_Destructible" NewResponse)
      (return))
    (:else
      (return))))

(fn SpawnDirectionalDestructionSphere
  (params (HitResult :type Hit%20Result%20Structure) (Radius :type Float%20%28double-precision%29) (HitProp :type Actor%20Object%20Reference) (VelocityNormal :type Vector) (Velocity :type Float%20%28double-precision%29) (ImpactVelocityMinMax :type Vector%202D%20Structure))
  ;[1 0.8203 0] Spawn directional destruction sphere, transform based on weapon swing data
  (Game|SpawnActorfromClass "/Game/PropDestructionSystem/DestructablePropsCore/BP_PropDestruction_PropDestructionField.BP_PropDestruction_PropDestructionField_C" (Math|Transform|MakeTransform (.Location (Collision|BreakHitResult HitResult)) (Math|Conversions|RotationFromXVector VelocityNormal)) "Undefined" 0 Velocity Radius (Utilities|Select :Index (Variables|Debug|GetDebugLevel) :NewEnumerator0 false :NewEnumerator1 true :NewEnumerator2 true) ImpactVelocityMinMax "NewEnumerator1" (Collision|GetOverlappingActors HitProp "/Game/PropDestructionSystem/DestructablePropsCore/BP_PropDestrution_Anchor.BP_PropDestrution_Anchor_C" :!class /Script/Engine.Actor) 0)
  (return))

(fn SpawnStandardDestructionSphere
  (params (SpawnTransform :type Transform) (ImpactVelocity :type Float%20%28single-precision%29) (SphereRadius :type Float%20%28single-precision%29) (ImpactVelocityMinMax :type Vector%202D%20Structure))
  (Game|SpawnActorfromClass "/Game/PropDestructionSystem/DestructablePropsCore/BP_PropDestruction_PropDestructionField.BP_PropDestruction_PropDestructionField_C" SpawnTransform "Undefined" 0 ImpactVelocity SphereRadius (Utilities|Select :Index (Variables|Debug|GetDebugLevel) :NewEnumerator0 false :NewEnumerator1 true :NewEnumerator2 true) ImpactVelocityMinMax "NewEnumerator1" 0 0)
  (return))

(fn TriggerWeaponTraceDestruction
  (params (HitActors :type Array%20of%20Actor%20Object%20References) (HitPropIndex :type Integer) (WeaponNotifyData :type F%20Prop%20Destruction%20Weapon%20Notify%20Data%20Structure%20%28by%20ref%29) (WeaponTraceData :type F%20Prop%20Destruction%20Weapon%20Trace%20Data%20Structure%20%28by%20ref%29) (HitResult :type Hit%20Result%20Structure) (VelocityNormal :type Vector) (Velocity :type Float%20%28double-precision%29) (ImpactVelocityMinMax :type Vector%202D%20Structure))
  (bind (_overridedestructionradius _overriddendestructionradius) (Utilities|Struct|BreakF_PropDestruction_Weapon_NotifyData WeaponNotifyData))
  (Utilities|FlowControl|Sequence
    (:then_0
      ;[0.7812 1 0] Spawn destruction spheres (only one per prop/per swing)
      (DestructionSpheres|SpawnDirectionalDestructionSphere HitResult (Math|Float|SelectFloat _overriddendestructionradius (Utilities|Struct|BreakF_PropDestruction_WeaponTraceData WeaponTraceData) _overridedestructionradius) (Utilities|Array|Get(acopy) HitActors HitPropIndex) VelocityNormal Velocity ImpactVelocityMinMax))
    (:then_1
      ;[1 0 0.5156] Set hit props to debug mode if debug is enabled
      (Utilities|DebugLevelGate
        (:Minimal
          _)
        (:Maximum
          _))
      (Class|BPIPropDestructionProp|BPISetPropDebug(Message) (.HitActor (Collision|BreakHitResult HitResult)) (Variables|Debug|GetDebugLevel))
      (return))))

(fn AddNeededComponentstoOwner
  (bind _returnvalue (Components|GetOwner))
  (bind _returnvalue_2 (Actor|GetComponentsByClass _returnvalue "/Game/PropDestructionSystem/DestructablePropsCore/BPC_PropDestruction_TraceComponent.BPC_PropDestruction_TraceComponent_C"))
  (if (Utilities|Array|IsEmpty _returnvalue_2)
    (bind _returnvalue_3 (Game|AddComponentbyClass _returnvalue "/Game/PropDestructionSystem/DestructablePropsCore/BPC_PropDestruction_TraceComponent.BPC_PropDestruction_TraceComponent_C"))
    (Variables|Default|SetOwnerTraceComponetRef _returnvalue_3)
    (else
      (Variables|Default|SetOwnerTraceComponetRef (Utilities|Array|Get(acopy) _returnvalue_2))))
  (return))

(fn UpdatePushForce
  (params (Condition :type Boolean))
  (if Condition
    (bind _pushspawnfieldref (Variables|PushForce|GetPushSpawnFieldRef)
      (:then
        (Variables|/Game/PropDestructionSystem/DestructablePropsCore/BP_PropDestruction_PropDestructionField.BP_PropDestruction_PropDestructionField_C|SetImpactVelocity _pushspawnfieldref (Math|Vector|VectorLength (Transformation|GetVelocity (Components|GetOwner))))
        (return))
      (:else))
    (else
      (return))))

(fn SpawnPushField
  (params (Condition :type Boolean))
  (bind _returnvalue (Components|GetOwner))
  (bind _returnvalue_2 (Transformation|GetActorTransform _returnvalue))
  (bind (_location _rotation) (Math|Transform|BreakTransform _returnvalue_2))
  (if Condition
    (bind _returnvalue_3 (Game|SpawnActorfromClass :Class "/Game/PropDestructionSystem/DestructablePropsCore/BP_PropDestruction_PropDestructionField.BP_PropDestruction_PropDestructionField_C" :SpawnTransform (Math|Transform|MakeTransform (+ _location (Variables|PushForce|GetPushForceSpawnOffset)) _rotation "1.000000,1.000000,1.000000") :CollisionHandlingOverride "Undefined" :ImpactVelocity (Math|Vector|VectorLength (Transformation|GetVelocity _returnvalue)) :Instigator 0))
    (bind _output_get (Variables|PushForce|SetPushSpawnFieldRef _returnvalue_3))
    (Transformation|AttachActorToActor _output_get (Components|GetOwner) "None" "KeepWorld" "KeepWorld" "KeepWorld" true)
    (return)
    (else
      (return))))
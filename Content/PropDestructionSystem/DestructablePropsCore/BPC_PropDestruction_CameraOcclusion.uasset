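; Actor component that drives a camera occlusion window, likely to keep its owner visible behind props in the prop destruction system.
; Each tick it writes the owner's location to a material parameter collection and sphere-traces from the player camera to that location plus an offset.
; The trace hit result smoothly interpolates the collection's CameraOcclusionWindow scalar between open and closed, leaving the visual effect to materials reading it.
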(event EventTick
  (params (DeltaSeconds :type Float%20%28single-precision%29))
  ;[0 0.9297 1] Update the location of the player
  (CallFunction|UpdateTargetLocation)
  ;[0.2422 0 1] Trace for intersecting objects
  (CallFunction|TraceforOcclusion (Variables|CameraOcclusion|GetOcclusionObjectTypes) DeltaSeconds))

(fn UpdateTargetLocation
  ;[0 1 0.5078] Update target location value in param collection
  (Rendering|Material|SetVectorParameterValue "/Game/PropDestructionSystem/DestructablePropsCore/MaterialLibrary/MPC_PropDestruction_CameraOcclusion.MPC_PropDestruction_CameraOcclusion" "TargetLocation" (Math|Conversions|ToLinearColor(Vector) (Transformation|GetActorLocation (Components|GetOwner))) :!class /Script/Engine.KismetMaterialLibrary)
  (return))

(fn TraceforOcclusion
  (params (ObjectTypes :type Array%20of%20EObjectTypeQuery%20Enums :default "ObjectTypeQuery1") (DeltaTime :type Float%20%28double-precision%29))
  ;[0.6875 1 0] Trace from camera to character
  (bind _returnvalue (Collision|MultiSphereTraceForObjects (Transformation|GetWorldLocation (Variables|/Script/Engine.PlayerCameraManager|GetTransformComponent (Game|GetPlayerCameraManager 0))) (+ (Transformation|GetActorLocation (Components|GetOwner)) (Variables|CameraOcclusion|GetTargetLocationOffset)) (Variables|CameraOcclusion|GetOcclusionTraceRadius) ObjectTypes false 0 "None"))
  ;[0 0.4844 1] Interp CameraOcclusionWindow value
  (bind _output_get (Variables|CameraOcclusion|SetCurrentOcclusionWindowValue (Math|Interpolation|FInterpTo (Variables|CameraOcclusion|GetCurrentOcclusionWindowValue) (Math|Float|SelectFloat 1.0 0.0 _returnvalue) DeltaTime (Variables|CameraOcclusion|GetOcclusionWindowInterpSpeed))))
  (Rendering|Material|SetScalarParameterValue "/Game/PropDestructionSystem/DestructablePropsCore/MaterialLibrary/MPC_PropDestruction_CameraOcclusion.MPC_PropDestruction_CameraOcclusion" "CameraOcclusionWindow" _output_get :!class /Script/Engine.KismetMaterialLibrary)
  (return))
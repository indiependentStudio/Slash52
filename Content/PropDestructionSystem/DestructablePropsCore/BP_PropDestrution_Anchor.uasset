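; Anchor field actor for the prop destruction system that forces destructible props inside its box to a static state.
; On construction it resets its field system and registers a dynamic-state command from a uniform integer field, culled outside a box falloff shaped by the AnchorBox transform.
; Actor rotation is locked to zero as a workaround for box falloff fields ignoring rotation.
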(fn ConstructionScript
  (Utilities|FlowControl|Sequence
    (:then_0
      ;[0 0.25 1] Keeps field rotation at 0 as box falloff fields do not currenly respect their rotation input, will remove this if an engine update fixes this
      (Transformation|SetActorRotation "0, 0, 0"))
    (:then_1
      ;[0.1484 0 1] Clears existing construction scripts
      (Class|FieldSystemComponent|ResetFieldSystem (Variables|Default|GetFieldSystem))
      ;[0 1 0.08594] Forces props in fields to static
      (Class|FieldSystemComponent|AddFieldCommand (Variables|Default|GetFieldSystem) true "Field_DynamicState" 0 (Field|SetCullingField (Variables|Default|GetCullingField) (Field|SetBoxFalloff (Variables|Default|GetBoxFalloff) 1.0 1.0 1.0 0.0 (Transformation|GetWorldTransform (Variables|Default|GetAnchorBox)) "Field_FallOff_None") (Field|SetUniformInteger (Variables|Default|GetUniformInteger) (Math|Conversions|ToInteger(Byte) (Variables|Default|GetDynamic%20State))) "Field_Culling_Outside")))))
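; Chaos field actor for prop destruction that applies transient strain and linear velocity fields to break and push destructible objects.
; FieldType selects per-tick strain, per-tick velocity, or a one-shot of both on spawn followed by delayed self-destruction.
; Impact velocity scales the magnitudes, optionally for strain.
; Velocity follows the Arrow's forward vector, culled by a radial falloff and filtered to destruction objects, with optional debug drawing.
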(event Custom|DestroyActor_Delayed
  (params (Delay :type Float%20%28single-precision%29))
  ;[1 0.5156 0] Wait fDelay seconds then destroy actor
  (Utilities|FlowControl|Delay Delay)
  (Actor|DestroyActor))

(event EventBeginPlay
  ;[0 0.7656 1] Fields that trigger once on spawn
  (switch Utilities|FlowControl|Switch|SwitchonE_PropDestruction_DestructionFieldTypes (Variables|Field|GetFieldType)
    (:NewEnumerator1
      (Utilities|FlowControl|Sequence
        (:then_0
          ;[0 0.7422 1] Spawn transient external strain field
          (CallFunction|SpawnTransientExternalStrainField))
        (:then_1
          ;[0.9922 0 1] Spawn transient linear velocity field
          (CallFunction|SpawnTransientLinearVelocityField))
        (:then_2
          ;[0 0.2734 1] Destroy field actor after given time
          (CallFunction|DestroyActorDelayed 1.0))))))

(event EventTick
  (params (DeltaSeconds :type Float%20%28single-precision%29))
  ;[0 1 0.625] Fields that trigger once per tick
  (switch Utilities|FlowControl|Switch|SwitchonE_PropDestruction_DestructionFieldTypes (Variables|Field|GetFieldType)
    (:NewEnumerator0
      ;[0 1 0.5547] Spawn Transient strain field on tick
      (CallFunction|SpawnTransientExternalStrainField))
    (:NewEnumerator2
      ;[0 1 0.9766] Spawn transient linear velocity field on tick
      (CallFunction|SpawnTransientLinearVelocityField))))

(fn ConstructionScript)

(fn MapImpactVelocity
  (params (Value :type Float%20%28double-precision%29) (InVec :type Vector%202D%20Structure) (OutMin :type Float%20%28double-precision%29) (OutMax :type Float%20%28double-precision%29))
  (bind (_x _y) (Math|Vector2D|BreakVector2D InVec))
  ;[1 1 1] Map impact velocity based on MinMax vector input
  (return (Math|Float|MapRangeClamped Value _x _y OutMin OutMax)))

(fn SpawnTransientExternalStrainField
  (Class|FieldSystemComponent|ApplyPhysicsField (Variables|Field|GetFieldSystemComponent) true "Field_ExternalClusterStrain" 0 (Field|SetRadialFalloff (Variables|Default|GetRadialFalloff) (select (Variables|Impact|GetbUseVelocityBasedFieldMagnitude) (CallFunction|MapImpactVelocity (Variables|Field|GetImpactVelocity) (Variables|Impact|GetImpactVelocityMinMax) 1e+05 5e+05) 5e+05) 0.0 1.0 0.0 (Variables|Field|GetSphereRadius) (Transformation|GetActorLocation) "Field_Falloff_Linear"))
  (if (Variables|Debug|GetbDebug)
    (Rendering|Debug|DrawDebugSphere (Transformation|GetActorLocation) (Variables|Field|GetSphereRadius) 12 "(R=1.000000,G=0.000000,B=0.000000,A=1.000000)" 0.0 1.0)
    (return)
    (else
      (return))))

(fn SpawnTransientLinearVelocityField
  (bind _returnvalue (Transformation|GetActorLocation))
  (bind _arrow (Variables|Default|GetArrow))
  (bind _returnvalue_2 (Math|Vector|GetForwardVector _arrow))
  (bind _returnvalue_3 (* _returnvalue_2 3e+01))
  (bind _returnvalue_4 (CallFunction|SetMetaDataProcessingFilter))
  (Class|FieldSystemComponent|ApplyPhysicsField (Variables|Field|GetFieldSystemComponent) true "Field_LinearVelocity" _returnvalue_4 (Field|SetCullingField (Variables|Default|GetCullingField) (Field|SetRadialFalloff (Variables|Default|GetRadialFalloff) (Variables|Field|GetImpactVelocity) 0.0 1.0 0.0 (Variables|Field|GetSphereRadius) (Transformation|GetActorLocation) "Field_Falloff_Linear") (Field|SetUniformVector (Variables|Default|GetUniformVector) (CallFunction|MapImpactVelocity (Variables|Field|GetImpactVelocity) (Variables|Impact|GetImpactVelocityMinMax) 5e+01 2e+02) (Math|Vector|GetForwardVector (Variables|Default|GetArrow))) "Field_Culling_Outside"))
  (if (Variables|Debug|GetbDebug)
    (Rendering|Debug|DrawDebugArrow (- _returnvalue _returnvalue_3) (+ _returnvalue _returnvalue_3) 1e+01 "(R=1.000000,G=1.000000,B=1.000000,A=1.000000)" 5.0 5.0)
    (Rendering|Debug|DrawDebugSphere (Transformation|GetActorLocation) (Variables|Field|GetSphereRadius) 12 "(R=1.000000,G=0.000000,B=0.000000,A=1.000000)" 5.0 1.0)
    (return)
    (else
      (return))))

(fn SetMetaDataProcessingFilter
  (return (Class|FieldSystemMetaDataFilter|SetMetaDataFilterType (Variables|Default|GetFieldSystemMetaDataFilter) "Field_Filter_All" "Field_Object_Destruction" "Field_Position_CenterOfMass")))
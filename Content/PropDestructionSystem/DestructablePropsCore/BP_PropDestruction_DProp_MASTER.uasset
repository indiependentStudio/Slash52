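; Master Blueprint for destructible Chaos Geometry Collection props, with empty events for children to override.
; The first break or an external wake swaps the proxy mesh for the collection and can wake overlapping props, with multicast init and first-break logic.
; Breaks spawn mass-gated particles and sounds.
; Timers use physics fields to keep pieces dynamic, sleep or disable them by time since last break, and optionally remove props by distance, time and screen visibility.
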(event OnChaosBreakEvent(GeometryCollection)
  (params (BreakEvent :type Chaos%20Break%20Event%20Structure%20%28by%20ref%29))
  ;[0 1 0.4844] Chaos break logic - required for prop functionality
  (Variables|Data|SetLastBreakEvent BreakEvent)
  (Utilities|FlowControl|Sequence
    (:then_0
      ;[1 0.9844 0] Disabled currently, info in function comments
      (Behaviour|SleepDisable|WakeDisabledObjects false)
      ;[0.3125 0 1] Function run on every break
      (OnEventFunctions|OnChaosBreakEvent))
    (:then_1
      ;[0 1 0.8125] Run initial break logic once
      (Utilities|InitialBreakGate
        (:false
          (CallFunction|MulticastDoInitialBreak))))
    (:then_2
      ;[0 1 0.7656] Run initilization functions once
      (Utilities|PropInitilizationGate
        (:Uninitilized
          (CallFunction|MulticastInitilizeProp))))))

(event OnChaosPhysicsCollision(GeometryCollection)
  (params (CollisionInfo :type Chaos%20Physics%20Collision%20Info%20Structure%20%28by%20ref%29))
  ;[0 1 0.8594] Chaos collision logic - no parent logic, disabled by default for optimization. To enable, set NotifyCollisions in GeometryCollection to True
  (ChildOverride|OnCollisionChildEvent CollisionInfo) ; For overriding in children
)

(event Custom|Multicast_DoInitialBreak
  ;[0 0.7187 1] Clients perform initil break logic
  (Variables|Flow|SetbInitiallyBroken true)
  ;[0.9219 1 0] Break event for overringing in children
  (ChildOverride|OnInitialBreakChildEvent (Variables|Data|GetLastBreakEvent))
  ;[0 1 0.1094] Spawn intial break sound, if enabled and set
  (Utilities|ShouldUseInitialBreakSound
    (:true
      (Visual|Sound|SpawnBreakSound (Variables|Data|GetLastBreakEvent) false (Variables|Sound|GetInitialBreakBreakSound) true 1e+02))))

(event Custom|Multicast_InitilizeProp
  ;[0 1 0.4141] Clients perform prop initilization logic
  (Utilities|FlowControl|Sequence
    (:then_0
      ;[0 0.08594 1] Wake prop
      (Initilization|InitialWake false)
      ;[1 0 0.2812] Wake event for overriding in children
      (ChildOverride|OnInitialWakeChildEvent)
      ;[1 0 0.2812] Start sleep/disable timer
      (Utilities|Time|SetTimerbyFunctionName 0 "ManageSleepDisable" (Variables|Behaviour|GetSleepDisableCheckInterval) true))
    (:then_1
      ;[1 0.8203 0] Force object state to dynamic
      (PhysicsFields|ForceObjectState "Chaos_Object_Dynamic" "(R=1.000000,G=0.705822,B=0.000000,A=1.000000)" 3.0 true))
    (:then_2
      ;[1 0 0.6797] Wake overlapping props if conditions are met
      (Utilities|ExternalPropWakeGate
        (:true
          (ExternalDPropWake|WakeOverlappingProps))))))

(event Custom|Server_DoInitialBreak
  ;[1 0.04688 0] Server notify clients to start prop break events
  (CallFunction|MulticastDoInitialBreak))

(event Custom|Server_InitilizeProp
  ;[1 0.04688 0] Server notify clients to start prop break events
  (CallFunction|MulticastInitilizeProp))

(event EventBPITriggerInitialWake
  ;[0.9453 0 1] External wake trigger event
  ;[0 1 0.7656] Run initilization functions once
  (Utilities|PropInitilizationGate
    (:Uninitilized
      (CallFunction|MulticastInitilizeProp))))

(event EventBeginPlay
  (switch Utilities|FlowControl|Switch|SwitchonE_PropDestruction_CollisionBehaviour (Variables|Behaviour|GetCollisionBehaviour)
    (:NewEnumerator0
      ;[0 1 0.08594] Update static mesh collision, causes issues if in construction script so needs to be here
      (Collision|SetCollisionEnabled (Variables|Default|GetProxyMesh) "QueryAndPhysics" :!label _label))
    (:NewEnumerator1
      (goto _label))
    (:NewEnumerator2
      (Collision|SetCollisionResponsetoChannel (Variables|Default|GetProxyMesh) "ECC_Pawn" "ECR_Ignore"))))

(fn ConstructionScript
  (bind (_origin _boxextent _sphereradius) (Utilities|GetGeometryCollectionBounds))
  (Utilities|FlowControl|Sequence
    (:then_0
      ;[1 0 0.1875] Loop through material overrides
      (if (> (Utilities|Array|Length (Variables|Material|GetMaterialOverrides)) 0)
        (for (_array_element _array_index) (Variables|Material|GetMaterialOverrides)
          (Utilities|FlowControl|Sequence
            (:then_0
              ;[0.5938 0 1] Update geo collection materials
              (if (and (Utilities|IsValid _array_element) (<= _array_index (Rendering|Material|GetNumMaterials (Variables|Default|GetGeometryCollection))))
                (Rendering|Material|SetMaterial (Variables|Default|GetGeometryCollection) _array_index _array_element)))
            (:then_1
              ;[1 0.09375 0] Update static mesh materials
              (if (and (Utilities|IsValid _array_element) (<= _array_index (Rendering|Material|GetNumMaterials (Variables|Default|GetProxyMesh))))
                (Rendering|Material|SetMaterial (Variables|Default|GetProxyMesh) _array_index _array_element)))))))
    (:then_1
      ;[0.4531 0 1] If geo collection is not breakable, set max cluster to 0 (intact collection)
      (if (not (Variables|Behaviour|GetbBreakable))
        (Variables|/Script/GeometryCollectionEngine.GeometryCollectionComponent|SetMaxClusterLevel (Variables|Default|GetGeometryCollection) 0)))
    (:then_2
      ;[0.8516 0 1] If prop does not wake other actors, hide wake box
      (Utilities|ExternalPropWakeGate
        (:false
          (Rendering|SetVisibility (Variables|Default|GetWakeBox) false false))))
    (:then_3
      ;[0 0.7187 1] Set geo collecion collision response based on desired collision behaviour
      (Collision|SetCollisionResponsetoChannel (Variables|Default|GetGeometryCollection) "ECC_Pawn" (Utilities|Select :Index (Variables|Behaviour|GetCollisionBehaviour) :NewEnumerator0 "ECR_Block" :NewEnumerator1 "ECR_Ignore" :NewEnumerator2 "ECR_Ignore")))
    (:then_4
      ;[0.7344 0 1] Disabled for potential deprication,, applies a contstruction field to set props intial state to static
      (if false
        (Class|FieldSystemComponent|ResetFieldSystem (Variables|Default|GetFieldSystem))
        (Class|FieldSystemComponent|AddFieldCommand (Variables|Default|GetFieldSystem) true "Field_DynamicState" (Class|FieldSystemMetaDataProcessingResolution|SetMetaDataaProcessingResolutionType (Variables|FieldSystemModifiers|GetFieldSystemMetaDataProcessingResolution) "Field_Resolution_Maximum") (Field|SetCullingField (Variables|FieldSystemModifiers|GetCullingField) (Field|SetRadialFalloff (Variables|FieldSystemModifiers|GetRadialFalloff_Culling) 1.0 1.0 1.0 0.0 (* (+ _sphereradius (Variables|Default|GetForceObjectStateAdditionalRadius)) (Math|Float|MapRangeClamped _sphereradius 2e+01 1e+01 1.0 4.0)) _origin "Field_FallOff_None") (Field|SetUniformInteger (Variables|FieldSystemModifiers|GetUniformInteger_ObjectState) (Math|Conversions|ToInteger(Byte) (Utilities|Enum|LiteralenumEObjectStateTypeEnum "Chaos_Object_Static"))) "Field_Culling_Outside"))))))

(fn InitialWake
  (params (bArtificialWake :type Boolean))
  (Utilities|FlowControl|Sequence
    (:then_0
      ;[0 1 0.03906] Flag prop as initilized
      (Variables|Flow|SetbInitilized true))
    (:then_1
      ;[0.2656 1 0] Destroy proxy mesh and make geo collection visible
      (Rendering|SetVisibility (Variables|Default|GetGeometryCollection) true false)
      (bind _proxymesh (Variables|Default|GetProxyMesh)
        (:then
          (Components|DestroyComponent _proxymesh))
        (:else)))
    (:then_2
      ;[0.9688 0 1] Start polling for removal if enabled
      (if (Utilities|Enum|NotEqual(Enum) (Variables|Removal|GetPropRemovalType) "NewEnumerator0")
        (Utilities|Time|SetTimerbyFunctionName 0 "PollForRemoval" (Variables|Removal|GetRemovalPollInterval) true)))
    (:then_3
      ;[0 0.1562 1] Remove any actors in the ActorsToRemoveOnWake array
      (for _array_element (Variables|ActorRemoval|GetActorsToRemoveOnWake)
        (Utilities|IsValid _array_element
          (:Is%20Valid
            (Actor|DestroyActor _array_element)))))
    (:then_4
      ;[0.1484 0 1] Debug: noitfy wake
      (Debug|DebugPrintDefaultWakeMessage bArtificialWake))))

(fn SpawnBreakParticle
  (params (ChaosBreakEvent :type Chaos%20Break%20Event%20Structure%20%28by%20ref%29))
  (for _array_element (Variables|Particle|GetBreakParticles)
    ;[1 0 0.4219] Only spawn particles if mass threshold + modifier is exceeded
    (if (>= (.Mass (Utilities|Struct|BreakChaosBreakEvent ChaosBreakEvent)) (+ (Variables|Particle|GetParticleMassThreshold) (.MassThresholdModifier (Utilities|Struct|BreakF_PropDestruction_ParticleData _array_element))))
      ;[1 0 0.3047] Spawn particle at location
      (bind _returnvalue (Niagara|SpawnSystematLocation (.Particle (Utilities|Struct|BreakF_PropDestruction_ParticleData _array_element)) (.Location (Utilities|Struct|BreakChaosBreakEvent ChaosBreakEvent))))
      ;[1 0 0.09375] Override colours
      (for _array_element_2 (.ColourOverrides (Utilities|Struct|BreakF_PropDestruction_ParticleData _array_element))
        (Effects|Components|ParticleSystem|SetColorParameter _returnvalue (.OverrideParamName (Utilities|Struct|BreakF_PropDestruction_ParticleOverrideData _array_element_2)) (.OverrideColour (Utilities|Struct|BreakF_PropDestruction_ParticleOverrideData _array_element_2))))))
  (return))

(fn HandleDisable
  (params (Physics%20Type :type EGeometryCollectionPhysicsTypeEnum%20Enum :default "Chaos_AngularVelocity"))
  ;[0.8281 1 0] Sleep or disable active geo collections
  (Class|GeometryCollectionComponent|ApplyPhysicsField (Variables|Default|GetGeometryCollection) true Physics%20Type (Class|FieldSystemMetaDataProcessingResolution|SetMetaDataaProcessingResolutionType (Variables|FieldSystemModifiers|GetFieldSystemMetaDataProcessingResolution) "Field_Resolution_Minimal") (Class|UniformScalar|SetUniformScalar (Variables|FieldSystemModifiers|GetUniformScalar_SleepDisable) (Math|Float|Square (Utilities|Select :Index Physics%20Type :Chaos_AngularVelocity 0.0 :Chaos_DynamicState 0.0 :Chaos_LinearVelocity 0.0 :Chaos_InitialAngularVelocity 0.0 :Chaos_InitialLinearVelocity 0.0 :Chaos_CollisionGroup 0.0 :Chaos_LinearForce 0.0 :Chaos_AngularTorque 0.0 :Chaos_DisableThreshold (Variables|Behaviour|SleepDisable|GetDisableThreshold) :Chaos_SleepingThreshold (Variables|Behaviour|SleepDisable|GetSleepThreshold) :Chaos_ExternalClusterStrain 0.0 :Chaos_InternalClusterStrain 0.0 :Chaos_LinearImpulse 0.0)))))

(fn OnChaosBreakEvent
  (bind _lastbreakevent (Variables|Data|GetLastBreakEvent))
  (bind (_component _location _velocity _angularvelocity _extents _mass) (Utilities|Struct|BreakChaosBreakEvent _lastbreakevent))
  (Utilities|FlowControl|Sequence
    (:then_0
      ;[1 0 0.4219] Spawn break particle
      (Visual|Particles|SpawnBreakParticle (Variables|Data|GetLastBreakEvent)))
    (:then_1
      ;[0.5469 1 0] Spawn break sound effect
      (if (Variables|Sound|GetbUseBreakSound)
        (Visual|Sound|SpawnBreakSound (Variables|Data|GetLastBreakEvent) true (Variables|Sound|GetBreakSound) false 1e+02)))
    (:then_2
      ;;[0 0.08594 1] Reset time since last break
      (Variables|Behaviour|SleepDisable|SetTimeSinceLastBreak 0.0))
    (:then_3
      ;[1 0.3984 0] Debug display break mass
      (Utilities|DebugLevelGate
        (:Maximum
          (Rendering|Debug|DrawDebugString _location (Utilities|String|ToString(Integer) (Math|Float|Truncate _mass)) 0 "(R=1.000000,G=0.886669,B=0.000000,A=1.000000)" 3.0))))))

(fn WakeOverlappingProps
  (bind _wakebox (Variables|Default|GetWakeBox))
  (bind _returnvalue (Transformation|GetWorldTransform _wakebox))
  ;[0.4062 0 1] Loop through every overlapping prop actor
  (bind _wakebox_2 (Variables|Default|GetWakeBox)
    (:then
      (for _array_element (Collision|GetOverlappingActors _wakebox_2 "BP_PropDestruction_DProp_MASTER_C" :!class /Script/Engine.PrimitiveComponent)
        (LocalVariables|SetWorkingWakeProp _array_element)
        ;[1 0 0.7734] Artificially wake each overlapping prop
        (Class|BPIPropDestructionProp|BPITriggerInitialWake(Message) (LocalVariables|GetWorkingWakeProp))
        ;[1 0.7031 0] Draw debug dot on woken props
        (Utilities|DebugLevelGate
          (:Maximum
            (Rendering|Debug|DrawDebugPoint (Transformation|GetActorLocation (LocalVariables|GetWorkingWakeProp)) 1e+01 "(R=0.353491,G=0.000000,B=1.000000,A=1.000000)" 3.0))))
      ;[1 0.2344 0] Flag hit prop as having woken other objects
      (Variables|Behaviour|SetbWokenOtherObjects true)
      ;[0 0.8828 1] Draw a debug box at the wake box
      (Utilities|DebugLevelGate
        (:Minimal
          _)
        (:Maximum
          _))
      (Rendering|Debug|DrawDebugBox (.location _returnvalue) (Components|Box|GetScaledBoxExtent _wakebox) "(R=1.000000,G=1.000000,B=1.000000,A=1.000000)" (.rotation _returnvalue) 2.0 2.0))
    (:else)))

(fn DebugPrintDefaultWakeMessage
  (params (bArtificialWake :type Boolean))
  (bind _geometrycollection (Variables|Default|GetGeometryCollection))
  (bind (_origin _boxextent _sphereradius) (Collision|GetComponentBounds _geometrycollection))
  (Utilities|DebugLevelGate
    (:No%20Debug
      (return))
    (:Minimal
      _)
    (:Maximum
      _))
  (Rendering|Debug|DrawDebugString (+ _origin (Math|Vector|MakeVector 0.0 0.0 _sphereradius)) (Utilities|String|Append (Utilities|GetDisplayName self) (Utilities|String|SelectString "artificially woken" "woken" bArtificialWake)) 0 (Math|Color|SelectColor "(R=1.000000,G=0.822458,B=0.000000,A=1.000000)" "(R=1.000000,G=0.074200,B=0.000000,A=1.000000)" bArtificialWake) 5.0)
  (return))

(fn ForceObjectState
  (params (DesiredObjectState :type EObjectStateTypeEnum%20Enum :default "Chaos_NONE") (DebugColour :type Linear%20Color%20Structure) (DebugDuration :type Float%20%28single-precision%29) (bRespectAnchors :type Boolean))
  (bind (_origin _boxextent _sphereradius) (Utilities|GetGeometryCollectionBounds))
  (bind (_origin_2 _boxextent_2 _sphereradius_2) (Utilities|GetGeometryCollectionBounds))
  (bind (_origin_3 _boxextent_3 _sphereradius_3) (Utilities|GetGeometryCollectionBounds))
  (bind (_origin_4 _boxextent_4 _sphereradius_4) (Utilities|GetGeometryCollectionBounds))
  (if (not (Math|Boolean|ANDBoolean (Utilities|Enum|Equal(Enum) DesiredObjectState "Chaos_Object_Dynamic") (Utilities|Array|IsNotEmpty (Collision|GetOverlappingActors "/Game/PropDestructionSystem/DestructablePropsCore/BP_PropDestrution_Anchor.BP_PropDestrution_Anchor_C" :!class /Script/Engine.Actor)) bRespectAnchors))
    ;[0 0.2266 1] Only apply within object bounds
    (Class|GeometryCollectionComponent|ApplyPhysicsField (Variables|Default|GetGeometryCollection) true "Chaos_DynamicState" (Class|FieldSystemMetaDataProcessingResolution|SetMetaDataaProcessingResolutionType (Variables|FieldSystemModifiers|GetFieldSystemMetaDataProcessingResolution) "Field_Resolution_Maximum") (Field|SetCullingField (Variables|FieldSystemModifiers|GetCullingField) (Field|SetRadialFalloff (Variables|FieldSystemModifiers|GetRadialFalloff_Culling) 1.0 0.0 1.0 0.0 (* (+ _sphereradius_2 (Variables|Default|GetForceObjectStateAdditionalRadius)) (Math|Float|MapRangeClamped _sphereradius_2 2e+01 1e+01 1.0 4.0)) _origin_2 "Field_FallOff_None") (Field|SetUniformInteger (Variables|FieldSystemModifiers|GetUniformInteger_ObjectState) (Math|Conversions|ToInteger(Byte) DesiredObjectState)) "Field_Culling_Outside"))
    ;[1 0.4688 0] Draw debug for state field
    (Utilities|DebugLevelGate
      (:No%20Debug
        (return))
      (:Minimal
        _)
      (:Maximum
        _))
    (Rendering|Debug|DrawDebugSphere _origin_3 _sphereradius_3 12 DebugColour DebugDuration 0.7)
    (return)
    (else
      ;[1 0.8672 0] Cull anchor fields from forced wake
      (Class|FieldSystemComponent|ApplyPhysicsField (Variables|Default|GetFieldSystem) true "Field_DynamicState" (Class|FieldSystemMetaDataProcessingResolution|SetMetaDataaProcessingResolutionType (Variables|FieldSystemModifiers|GetFieldSystemMetaDataProcessingResolution) "Field_Resolution_Maximum") (Field|SetCullingField (Variables|FieldSystemModifiers|GetCullingField) (Field|SetOperatorField (Variables|Default|GetOperatorField) 1.0 (Field|SetBoxFalloff (Variables|Default|GetAnchorBoxFalloffCulling) 1.0 1.0 1.0 0.0 (Transformation|GetActorTransform (Utilities|Array|Get(acopy) (Collision|GetOverlappingActors "/Game/PropDestructionSystem/DestructablePropsCore/BP_PropDestrution_Anchor.BP_PropDestrution_Anchor_C" :!class /Script/Engine.Actor))) "Field_FallOff_None") (Field|SetRadialFalloff (Variables|FieldSystemModifiers|GetRadialFalloff_Culling) 1.0 0.0 1.0 0.0 (* (+ _sphereradius (Variables|Default|GetForceObjectStateAdditionalRadius)) (Math|Float|MapRangeClamped _sphereradius 2e+01 1e+01 1.0 4.0)) _origin "Field_FallOff_None") "Field_Substract") (Field|SetUniformInteger (Variables|FieldSystemModifiers|GetUniformInteger_ObjectState) (Math|Conversions|ToInteger(Byte) DesiredObjectState)) "Field_Culling_Outside"))
      ;[1 0.4688 0] Draw debug for state field
      (Utilities|DebugLevelGate
        (:No%20Debug
          (return))
        (:Minimal
          _)
        (:Maximum
          _))
      (Rendering|Debug|DrawDebugSphere _origin_4 _sphereradius_4 12 DebugColour DebugDuration 0.7)
      (return))))

(fn GetGeometryCollectionBounds
  (bind _geometrycollection (Variables|Default|GetGeometryCollection))
  (bind (_origin _boxextent _sphereradius) (Collision|GetComponentBounds _geometrycollection))
  (return _origin _boxextent _sphereradius))

(fn OnInitialBreakChildEvent
  (params (BreakEvent :type Chaos%20Break%20Event%20Structure))
  (return))

(fn OnInitialWakeChildEvent
  (return))

(fn DebugPrintSleepWakeString
  (params (Text :type String) (TextColor :type Linear%20Color%20Structure))
  ;[1 1 1] Print message above actor source
  (Rendering|Debug|DrawDebugString (+ (Transformation|GetWorldLocation (Variables|Default|GetGeometryCollection)) "0,0,100.000000") Text 0 TextColor 0.15)
  (return))

(fn ManageSleepDisable
  ;[1 1 1] Only increse value if time incremented is less than removal threshold threshold
  (if (<= (Variables|Behaviour|SleepDisable|GetTimeSinceLastBreak) (Variables|Removal|GetRemovalTimeThreshold))
    ;[1 1 1] Increase time since last break by the timer interval
    (Variables|Behaviour|SleepDisable|SetTimeSinceLastBreak (+ (Variables|Behaviour|SleepDisable|GetTimeSinceLastBreak) (Variables|Behaviour|GetSleepDisableCheckInterval))))
  (Utilities|GetDisableAllowances
    (:Disable
      ;[1 1 1] If time since last break exceeds disable threshold, disable
      (Behaviour|SleepDisable|HandleDisable "Chaos_DisableThreshold")
      (Utilities|DebugLevelGate
        (:Maximum
          (Debug|DebugPrintSleepWakeString "Disabling" "(R=0.000000,G=1.000000,B=0.760236,A=1.000000)"))))
    (:Sleep
      ;[1 1 1] If time since last break exceeds sleep threshold but not disable threshold, sleep
      (Behaviour|SleepDisable|HandleDisable "Chaos_SleepingThreshold")
      (Utilities|DebugLevelGate
        (:Maximum
          (Debug|DebugPrintSleepWakeString "Sleeping" "(R=0.000000,G=1.000000,B=0.085570,A=1.000000)"))))
    (:Dynamic
      ;[1 1 1] If time since last break does not exceed any threshold and the object has been initilized, force it to be dynamic
      (PhysicsFields|ForceObjectState "Chaos_Object_Dynamic" "(R=1.000000,G=0.000000,B=0.816903,A=1.000000)" 0.0 true)
      (Utilities|DebugLevelGate
        (:Maximum
          (Debug|DebugPrintSleepWakeString "Setting Dynamic" "(R=1.000000,G=0.029966,B=0.000000,A=1.000000)"))))))

(fn WakeDisabledObjects
  (params (bEnabled :type Boolean))
  (bind (_origin _boxextent _sphereradius) (Utilities|GetGeometryCollectionBounds))
  (bind (_origin_2 _boxextent_2 _sphereradius_2) (Utilities|GetGeometryCollectionBounds))
  ;[0 1 0.4844] Does not currently function
  (if bEnabled
    ;;[0 1 0.5781] Only run when disable time threshold has been exceeded
    (if (> (Variables|Behaviour|SleepDisable|GetTimeSinceLastBreak) (Variables|Behaviour|SleepDisable|GetDisableTimeThreshold))
      ;;[1 0.7266 0] Intended to reawaken disabled particles but literally makes everything in the field explode. The ActivateDisabled function does not seem to work as intended and appears to ignore all rules set in the geo collection for clustering, damage thresholds, meta data filters etc.
      (Class|FieldSystemComponent|ApplyPhysicsField (Variables|Default|GetFieldSystem) true "Field_ActivateDisabled" (Class|FieldSystemMetaDataFilter|SetMetaDataFilterType (Variables|Default|GetFieldSystemMetaDataFilter) "Field_Filter_Disabled" "Field_Object_Destruction" "Field_Position_CenterOfMass") (Field|SetCullingField (Variables|FieldSystemModifiers|GetCullingField) (Field|SetRadialFalloff (Variables|FieldSystemModifiers|GetRadialFalloff_Culling) 1.0 0.0 1.0 0.0 _sphereradius_2 _origin_2 "Field_FallOff_None") (Field|SetUniformInteger (Variables|FieldSystemModifiers|GetUniformInteger_ObjectState) 0) "Field_Culling_Outside"))
      ;;;[0.6875 0 1] Debug
      (Utilities|DebugLevelGate
        (:No%20Debug
          (return))
        (:Minimal
          _)
        (:Maximum
          _))
      (Rendering|Debug|DrawDebugSphere _origin _sphereradius 12 "(R=1.000000,G=0.000000,B=0.000000,A=1.000000)" 1e+01 1.0)
      (Development|PrintString (Utilities|String|Append (Utilities|GetDisplayName self) " attempting re-enable"))
      (return)
      (else
        _)))
  (return))

(fn PollforRemoval
  (switch Utilities|FlowControl|Switch|SwitchonE_PropDestruction_RemovalTypes (Variables|Removal|GetPropRemovalType)
    (:NewEnumerator0
      ;[0 0.6484 1] If removal is disabled, do nothing
      (return))
    (:NewEnumerator1
      ;[1 0 0.9141] If removal distance is exceeded
      (Utilities|RemovalDistanceExceeded
        (:true
          (Behaviour|Removal|TryRemoveProp))
        (:false
          _))
      (return))
    (:NewEnumerator2
      ;[0.5234 0 1] If removal time is exceeded
      (Utilities|RemovalTimeExceeded
        (:true
          (Behaviour|Removal|TryRemoveProp))
        (:false
          _))
      (return))
    (:NewEnumerator3
      ;[1 0 0.9375] If removal time and removal distance is exceeded
      (Utilities|RemovalDistanceExceeded
        (:true
          (Utilities|RemovalTimeExceeded
            (:true
              (Behaviour|Removal|TryRemoveProp))
            (:false
              _)))
        (:false
          _))
      (return))))

(fn GetDistancetoPlayer
  (return (Transformation|GetDistanceTo self (Game|GetPlayerCharacter 0))))

(fn TryRemoveProp
  (if (Variables|Removal|GetbRequireOffScreenForRemovals)
    ;[1 1 1] Destroy prop actor if it is off screen
    (if (Behaviour|Removal|IsProponScreen)
      (return false)
      (else
        (Actor|DestroyActor)
        (return true)))
    (else
      ;[1 1 1] If off screen is not required, destroy without check
      (Actor|DestroyActor)
      (return true))))

(fn IsProponScreen
  (bind _returnvalue (Game|GetPlayerController 0))
  (bind _returnvalue_2 (Transformation|GetActorLocation))
  (bind _returnvalue_3 (Viewport|GetViewportSize))
  (bind _screenlocation (Class|PlayerController|ProjectWorldLocationtoScreen _returnvalue _returnvalue_2 true))
  (bind (_x _y) (Math|Vector2D|BreakVector2D _returnvalue_3))
  (bind (_x_2 _y_2) (Math|Vector2D|BreakVector2D _screenlocation))
  (return (Math|Boolean|ANDBoolean (> _x_2 0.0) (> _y_2 0.0) (< _x_2 _x) (< _y_2 _y))))

(fn SpawnBreakSound
  (params (ChaosBreakEvent :type Chaos%20Break%20Event%20Structure%20%28by%20ref%29) (bUseMassThreshold :type Boolean) (Sound :type Sound%20Base%20Object%20Reference) (bSetSoundPriority :type Boolean) (NewSoundPriority :type Float%20%28double-precision%29))
  (bind _soundmassthresholdminmax (Variables|Sound|GetSoundMassThresholdMinMax))
  (bind (_location _extents _mass) (Utilities|Struct|BreakChaosBreakEvent ChaosBreakEvent))
  ;[1 0.1172 0] Play sound directly if not using mass threshold
  (if (not bUseMassThreshold)
    _
    (else
      ;[0.2656 1 0] Gate play by min mass
      (if (>= (.Mass (Utilities|Struct|BreakChaosBreakEvent ChaosBreakEvent)) (.X (Math|Vector2D|BreakVector2D (Variables|Sound|GetSoundMassThresholdMinMax))))
        _
        (else
          (return false 0)))))
  ;[0.2656 0 1] Map and spawn sound
  (bind _returnvalue (Audio|SpawnSoundatLocation Sound _location "0, 0, 0" (Visual|Sound|MapSoundValue _mass _soundmassthresholdminmax (Variables|Sound|GetSoundMassVolumeOutputMinMax) (Variables|Sound|GetbUseSoundMassVolumeMapping) 1.0) (Visual|Sound|MapSoundValue _mass _soundmassthresholdminmax (Variables|Sound|GetSoundMassPitchOutputMinMax) (Variables|Sound|GetbUseSoundMassPitchMapping) 1.0) 0.0 (Variables|Sound|GetBreakSoundAttenuation) (Variables|Sound|GetBreakSoundConcurrency)))
  ;[1 0.7266 0] Adjusts the sound priority to NewSoundPriority if bSetSoundPriority is true and the sound spawned correctly
  (if (and bSetSoundPriority (Utilities|IsValid _returnvalue))
    (Variables|/Script/Engine.AudioComponent|SetPriority _returnvalue NewSoundPriority))
  (return (Utilities|IsValid _returnvalue) _returnvalue))

(fn MapSoundValue
  (params (InValue :type Float%20%28double-precision%29) (InMinMax :type Vector%202D%20Structure) (OutMinMax :type Vector%202D%20Structure) (bUseMappedValue :type Boolean) (UnmappedDefaultValue :type Float%20%28double-precision%29))
  (bind (_x _y) (Math|Vector2D|BreakVector2D OutMinMax))
  (bind (_x_2 _y_2) (Math|Vector2D|BreakVector2D InMinMax))
  ;[1 0 0.6797] Map sound value to an input range, or output a default value if bUseMappedValue is disabled
  (return (Math|Float|SelectFloat (Math|Float|MapRangeClamped InValue _x_2 _y_2 _x _y) UnmappedDefaultValue bUseMappedValue)))

(fn OnCollisionChildEvent
  (params (InCollisionInfo :type Chaos%20Physics%20Collision%20Info%20Structure))
  ;[1 0.9609 0] For overriding in children, no parent logic
  (return))

(fn BPISetPropDebug
  (params (NewDebug :type E_PropDestruction_DebugLevel%20Enum :default "NewEnumerator0"))
  ;[0 0.3437 1] Set prop debug level
  (Variables|Debug|SetDebugLevel NewDebug)
  (return true))
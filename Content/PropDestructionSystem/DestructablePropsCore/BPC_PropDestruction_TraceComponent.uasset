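; Actor component that runs melee weapon hit traces to destroy props and react to hard surfaces.
; While an anim notify enables it, Tick builds socket sphere or bounds box traces, subdividing each frame's swing to fill gaps and computing velocity.
; Each actor is hit once per swing, then routed by tag: Destructible Prop feeds velocity to the owner's Destructor component; Hard Surface optionally plays sparks, sound and an angle-gated montage.
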(event EventTick
  (params (DeltaSeconds :type Float%20%28single-precision%29))
  (Utilities|WeaponTraceActive
    (:True
      (Utilities|FlowControl|Sequence
        (:then_0
          ;[0 0.6016 1] Update weapon trace data
          (Variables|WeaponTrace|SetLastWeaponTraceData (WeaponTrace|GetWeaponMeshTraceData (Variables|WeaponTrace|GetWeaponHitboxExtension))))
        (:then_1
          ;[0 1 0.01562] Calculate swing data
          (bind (_weaponvelocity _weaponvelocitynormal _tracepoints _bfailed) (WeaponTrace|CalculateWeaponSwingData))
          (if (not _bfailed)
            (Variables|WeaponVelocity|SetWeapon%20Velocity%20Normal _weaponvelocitynormal)
            (Variables|WeaponVelocity|SetWeapon%20Velocity _weaponvelocity)
            ;[0 0.2734 1] Trace once per radial division of the weapon distance travelled
            (for _array_element _tracepoints
              ;[0.05469 0 1] Trace for destructable objects
              (bind (_outhit _returnvalue) (WeaponTrace|WeaponTraceforObjects (Utilities|Struct|BreakF_PropDestruction_Weapon_NotifyData (Variables|WeaponTrace|GetLatestWeaponNotifyData)) _array_element (Variables|WeaponTrace|GetLastWeaponTraceData) (Transformation|GetWorldRotation (Variables|Default|GetLastWeaponMeshRef)) (Variables|WeaponTrace|GetTraceActorsToIgnore)))
              ;;[1 0.1875 0] Could check better
              (if (and _returnvalue (Utilities|IsValid (.HitActor (Collision|BreakHitResult _outhit))))
                (Variables|WeaponTrace|SetLastValidHitResult _outhit)
                ;[0 1 0.3203] Only effect props once per swing, array cleared by anim notify
                (bind _returnvalue_2 (Utilities|Array|AddUnique (Variables|WeaponTrace|GetTraceActorsToIgnore) (.HitActor (Collision|BreakHitResult (Variables|WeaponTrace|GetLastValidHitResult)))))
                (if (!= _returnvalue_2 -1)
                  (Variables|WeaponTrace|SetLastHitActorIndex _returnvalue_2)
                  (Utilities|FlowControl|Sequence
                    (:then_0
                      ;[0 0.08594 1] Get working actor
                      (Utilities|IsValid (Utilities|Array|Get(acopy) (Variables|WeaponTrace|GetTraceActorsToIgnore) (Variables|WeaponTrace|GetLastHitActorIndex))
                        (:Is%20Valid
                          (bind _output_get (Variables|WeaponTrace|SetActiveLastHitActor (Utilities|Array|Get(acopy) (Variables|WeaponTrace|GetTraceActorsToIgnore) (Variables|WeaponTrace|GetLastHitActorIndex))))
                          ;[0.3828 1 0] Loop through actor tags
                          (for _array_element_2 (Variables|/Script/Engine.Actor|GetTags _output_get)
                            (WeaponHitResult|ForEachHitActorTags _array_element_2)))))))))))))))

(event EventBeginPlay
  (Init|SetOwnerRefs))

(fn ResetWeaponData
  ;[0 1 0.9766] Reset variables related to the gathering of the weapon swing/trace data
  (Variables|WeaponTrace|SetLastWeaponEndLocation "0, 0, 0")
  (Variables|WeaponVelocity|SetLastHitTotalDeltVelocity 0.0)
  (return))

(fn ManageWeaponTrace
  (params (StartTrace :type Boolean) (NewWeaponNotifyData :type F%20Prop%20Destruction%20Weapon%20Notify%20Data%20Structure))
  ;[0.1719 1 0] Called by anim notify
  ;[0.6641 0 1] Set weapon wake destructables
  (bind _output_get (Variables|WeaponTrace|SetbWeaponTraceActive StartTrace))
  (if _output_get
    ;[0.9219 0 1] Update trace data
    (Variables|WeaponTrace|SetLatestWeaponNotifyData NewWeaponNotifyData)
    ;[1 0.02344 0] If starting trace, set relevant weapon mesh ref
    (bind _weaponmeshcomponent (Class|BPIPropDestructionSource|BPIGetRelevantComponents(Message) (Components|GetOwner)))
    (Variables|Default|SetLastWeaponMeshRef _weaponmeshcomponent)
    (return)
    (else
      ;[0 1 0.1562] If ending trace, clear trace data
      (Utilities|Array|Clear (Variables|WeaponTrace|GetTraceActorsToIgnore))
      (WeaponTrace|ResetWeaponData)
      (return))))

(fn SetOwnerRefs
  ;[1 0 0.3984] Set references to the owning actor's skeletal mesh and capsule collision components
  (bind (_weaponmeshcomponent _skeletalmeshcomponent _capsulecomponent) (Class|BPIPropDestructionSource|BPIGetRelevantComponents(Message) (Components|GetOwner)))
  (Utilities|FlowControl|Sequence
    (:then_0
      (Utilities|IsValid _skeletalmeshcomponent
        (:Is%20Valid
          (Variables|Default|SetOwnerSkeletalMeshRef _skeletalmeshcomponent))))
    (:then_1
      (Utilities|IsValid _capsulecomponent
        (:Is%20Valid
          (Variables|Default|SetCapsule%20Component _capsulecomponent))))
    (:then_2
      (Init|InitPropDestrucionComponentRef))))

(fn InitPropDestrucionComponentRef
  (bind _returnvalue (Components|GetOwner))
  (bind _returnvalue_2 (Actor|GetComponentsByClass _returnvalue "/Game/PropDestructionSystem/DestructablePropsCore/BPC_PropDestruction_DestructorComponent.BPC_PropDestruction_DestructorComponent_C"))
  (if (Utilities|Array|IsNotEmpty _returnvalue_2)
    (Variables|Default|SetOwnerPropDestructionComponentRef (Utilities|Array|Get(acopy) _returnvalue_2))
    (Utilities|Array|Add (Variables|WeaponTrace|GetObjectsToTraceFor) "ObjectTypeQuery6"))
  (return))

(fn GetWeaponMeshTraceData
  (params (BoxHitboxExtension :type Float%20%28double-precision%29))
  (bind _lastweaponmeshref (Variables|Default|GetLastWeaponMeshRef))
  (bind _lastweaponmeshref_2 (Variables|Default|GetLastWeaponMeshRef))
  (bind _lastweaponmeshref_3 (Variables|Default|GetLastWeaponMeshRef))
  (bind _returnvalue (Transformation|GetSocketLocation _lastweaponmeshref "WeaponEnd"))
  (bind (_origin _boxextent _sphereradius) (Collision|GetComponentBounds _lastweaponmeshref_3))
  (bind _returnvalue_2 (Transformation|GetSocketLocation _lastweaponmeshref_2 "WeaponStart"))
  (switch Utilities|FlowControl|Switch|SwitchonE_PropDestruction_WeaponTraceMethods (Utilities|Struct|BreakF_PropDestruction_Weapon_NotifyData (Variables|WeaponTrace|GetLatestWeaponNotifyData))
    (:NewEnumerator0
      ;[0 0.4375 1] Bounds based box trace generation (less reliable)
      ;;[0.7578 1 0] Get mean local bounds of mesh
      (bind _asstatic_mesh_component (Utilities|Casting|CastToStaticMeshComponent (Variables|Default|GetLastWeaponMeshRef)))
      ;;[1 0.8203 0] Calculate start, end and halfsize from bounds origin
      (return (Utilities|Struct|MakeF_PropDestruction_WeaponTraceData (- _origin (* (.z (+ (/ (+ (Math|Vector|VectorGetAbs (.Min (Components|StaticMesh|GetLocalBounds _asstatic_mesh_component))) (Math|Vector|VectorGetAbs (.Max (Components|StaticMesh|GetLocalBounds _asstatic_mesh_component)))) 2.0) BoxHitboxExtension)) (Math|Vector|GetUpVector (Variables|Default|GetLastWeaponMeshRef)))) (+ (* (.z (+ (/ (+ (Math|Vector|VectorGetAbs (.Min (Components|StaticMesh|GetLocalBounds _asstatic_mesh_component))) (Math|Vector|VectorGetAbs (.Max (Components|StaticMesh|GetLocalBounds _asstatic_mesh_component)))) 2.0) BoxHitboxExtension)) (Math|Vector|GetUpVector (Variables|Default|GetLastWeaponMeshRef))) _origin) (Math|Vector|MakeVector (.x (+ (/ (+ (Math|Vector|VectorGetAbs (.Min (Components|StaticMesh|GetLocalBounds _asstatic_mesh_component))) (Math|Vector|VectorGetAbs (.Max (Components|StaticMesh|GetLocalBounds _asstatic_mesh_component)))) 2.0) BoxHitboxExtension)) (.y (+ (/ (+ (Math|Vector|VectorGetAbs (.Min (Components|StaticMesh|GetLocalBounds _asstatic_mesh_component))) (Math|Vector|VectorGetAbs (.Max (Components|StaticMesh|GetLocalBounds _asstatic_mesh_component)))) 2.0) BoxHitboxExtension)) 0.0) _sphereradius _sphereradius)))
    (:NewEnumerator2
      ;[1 0 0.4922] Socket based capsule generation (more reliable) requires sockets "WeaponStart" and "WeaponEnd" on weapon component
      (return (Utilities|Struct|MakeF_PropDestruction_WeaponTraceData _returnvalue_2 _returnvalue "0.000000,0.000000,0.000000" (Utilities|Struct|BreakF_PropDestruction_Weapon_NotifyData (Variables|WeaponTrace|GetLatestWeaponNotifyData)) (Math|Vector|Distance(Vector) _returnvalue_2 _returnvalue))))
    (:NewEnumerator1
      ;[0 0.5781 1] Reserved state for custom trace methods
      (return (Utilities|Struct|MakeF_PropDestruction_WeaponTraceData "0.000000,0.000000,0.000000" "0.000000,0.000000,0.000000")))))

(fn WeaponTraceforObjects
  (params (TraceType :type E_PropDestruction_WeaponTraceMethods%20Enum :default "NewEnumerator0") (TracePoints :type F%20Prop%20Destruction%20Weapon%20Trace%20Points%20Structure) (TraceData :type F%20Prop%20Destruction%20Weapon%20Trace%20Data%20Structure) (BoxOrientation :type Rotator) (ActorsToIgnore :type Array%20of%20Actor%20Object%20References))
  (bind (_tracestart _traceend) (Utilities|Struct|BreakF_PropDestruction_WeaponTracePoints TracePoints))
  (bind (_tracestart_2 _traceend_2) (Utilities|Struct|BreakF_PropDestruction_WeaponTracePoints TracePoints))
  (Utilities|FlowControl|Sequence
    (:then_0
      ;[0.4062 0 1] Initially set debug type for traces
      (LocalVariables|SetDebugType (Utilities|Select :Index (Variables|Debug|GetDebugLevel) :NewEnumerator0 "None" :NewEnumerator1 "ForOneFrame" :NewEnumerator2 "ForDuration")))
    (:then_1
      ;[1 0.2109 0] Trace type based on anim notify
      (switch Utilities|FlowControl|Switch|SwitchonE_PropDestruction_WeaponTraceMethods TraceType
        (:NewEnumerator0
          ;[1 0 0.1641] Box trace
          (bind (_outhit _returnvalue) (Class|KismetSystemLibrary|BoxTraceSingleforObjects _tracestart_2 _traceend_2 (Utilities|Struct|BreakF_PropDestruction_WeaponTraceData TraceData) BoxOrientation (Variables|WeaponTrace|GetObjectsToTraceFor) true ActorsToIgnore (LocalVariables|GetDebugType) true "(R=1.000000,G=0.000000,B=0.000000,A=1.000000)" "(R=0.000000,G=1.000000,B=0.000000,A=1.000000)" 0.0))
          (return _outhit _returnvalue))
        (:NewEnumerator2
          ;[0.7812 1 0] Capsule trace
          (bind (_outhit_2 _returnvalue_2) (Collision|SphereTraceForObjects _tracestart _traceend (Utilities|Struct|BreakF_PropDestruction_WeaponTraceData TraceData) (Variables|WeaponTrace|GetObjectsToTraceFor) true ActorsToIgnore (LocalVariables|GetDebugType) true "(R=1.000000,G=0.000000,B=0.000000,A=1.000000)" "(R=0.000000,G=1.000000,B=0.000000,A=1.000000)" 0.0))
          (return _outhit_2 _returnvalue_2))
        (:NewEnumerator1
          ;[0 1 0.5547] Add custom trace logic if needed
          (return "" false))))))

(fn DrawWeaponSwingDebug
  (bind _weaponvelocityrangeclamped (Variables|WeaponVelocity|GetWeaponVelocityRangeClamped))
  (if (Class|KismetMathLibrary|NotEqualExactlyVectorVector "0, 0, 0" (Variables|WeaponTrace|GetLastWeaponEndLocation))
    (Rendering|Debug|DrawDebugArrow (Variables|WeaponTrace|GetLastWeaponEndLocation) (.TraceEnd (Utilities|Struct|BreakF_PropDestruction_WeaponTraceData (Variables|WeaponTrace|GetLastWeaponTraceData))) 0.0 (Math|Color|Lerp(LinearColor) "(R=1.000000,G=0.000000,B=0.000000,A=1.000000)" "(R=0.000000,G=1.000000,B=0.082718,A=1.000000)" (Math|Float|MapRangeClamped (Math|Vector|Distance(Vector) (Variables|WeaponTrace|GetLastWeaponEndLocation) (.TraceEnd (Utilities|Struct|BreakF_PropDestruction_WeaponTraceData (Variables|WeaponTrace|GetLastWeaponTraceData)))) (.x _weaponvelocityrangeclamped) (.y _weaponvelocityrangeclamped) 0.0 1.0)) (Variables|Debug|GetDebugDrawTime) 1.0)
    (return)))

(fn GetDebugColourfromVelocity
  (params (Value :type Float%20%28double-precision%29))
  (bind _weaponvelocityrangeclamped (Variables|WeaponVelocity|GetWeaponVelocityRangeClamped))
  ;[0 0.5078 1] Lerp red to green for debug draws
  (return (Math|Color|Lerp(LinearColor) "(R=1.000000,G=0.000000,B=0.000000,A=1.000000)" "(R=0.000000,G=1.000000,B=0.082718,A=1.000000)" (Math|Float|MapRangeClamped Value (.x _weaponvelocityrangeclamped) (.y _weaponvelocityrangeclamped) 0.0 1.0))))

(fn ProcessWeaponVelocity
  (params (Velocity :type Float%20%28double-precision%29))
  (bind _latestweaponnotifydata (Variables|WeaponTrace|GetLatestWeaponNotifyData))
  (bind _alloweddeltvelocityperswing (Variables|WeaponVelocity|GetAllowedDeltVelocityPerSwing))
  (bind _preinterpvelocitymultiplier (Utilities|Struct|BreakF_PropDestruction_Weapon_NotifyData _latestweaponnotifydata))
  (bind _returnvalue (* Velocity _preinterpvelocitymultiplier))
  ;[1 0 0.04688] Multiply velocity by per interp multiplier (set by anim notify) and clamp before the max delt velocity is reached
  (return (select (> (+ _alloweddeltvelocityperswing (+ _returnvalue (Variables|WeaponVelocity|GetLastHitTotalDeltVelocity))) _alloweddeltvelocityperswing) _returnvalue 0.0)))

(fn CalculateWeaponSwingData
  (bind _lastweapontracedata (Variables|WeaponTrace|GetLastWeaponTraceData))
  (bind _lastweapontracedata_2 (Variables|WeaponTrace|GetLastWeaponTraceData))
  (bind _lastweapontracedata_3 (Variables|WeaponTrace|GetLastWeaponTraceData))
  (bind _lastweapontracedata_4 (Variables|WeaponTrace|GetLastWeaponTraceData))
  (bind (_tracestart _traceend) (Utilities|Struct|BreakF_PropDestruction_WeaponTraceData _lastweapontracedata_3))
  (bind (_tracestart_2 _traceend_2) (Utilities|Struct|BreakF_PropDestruction_WeaponTraceData _lastweapontracedata))
  (bind (_tracestart_3 _traceend_3) (Utilities|Struct|BreakF_PropDestruction_WeaponTraceData _lastweapontracedata_2))
  (bind (_tracestart_4 _traceend_4) (Utilities|Struct|BreakF_PropDestruction_WeaponTraceData _lastweapontracedata_4))
  ;[0 1 0.3672] Check if the last velocity normal location has been set yet
  (if (Class|KismetMathLibrary|NotEqualExactlyVectorVector "0, 0, 0" (Variables|WeaponTrace|GetLastWeaponEndLocation))
    (Utilities|FlowControl|Sequence
      (:then_0
        ;[1 0 0.6094] Calculate and set weapon velocity
        (LocalVariables|SetWeaponDistanceTravelled (Math|Vector|Distance(Vector) (Variables|WeaponTrace|GetLastWeaponEndLocation) (.TraceEnd (Utilities|Struct|BreakF_PropDestruction_WeaponTraceData (Variables|WeaponTrace|GetLastWeaponTraceData)))))
        (LocalVariables|SetNewWeaponVelocity (/ (Math|Vector|Distance(Vector) (Variables|WeaponTrace|GetLastWeaponEndLocation) (.TraceEnd (Utilities|Struct|BreakF_PropDestruction_WeaponTraceData (Variables|WeaponTrace|GetLastWeaponTraceData)))) (Utilities|Time|GetWorldDeltaSeconds))))
      (:then_1
        ;[0 0.7891 1] Calculate and set weapon velocity normal (direction)
        (LocalVariables|SetNewWeaponVelocityNormal (Math|Vector|GetUnitDirection(Vector) (Variables|WeaponTrace|GetLastWeaponEndLocation) (.TraceStart (Utilities|Struct|BreakF_PropDestruction_WeaponTraceData (Variables|WeaponTrace|GetLastWeaponTraceData))))))
      (:then_2
        ;[0 1 0.08594] Calculate trace increment points
        (if (> (Math|Float|Round (/ (LocalVariables|GetWeaponDistanceTravelled) (Utilities|Struct|BreakF_PropDestruction_Weapon_NotifyData (Variables|WeaponTrace|GetLatestWeaponNotifyData)))) 0)
          ;;[0 0.5547 1] If there are gaps in trace, run trace in increments based on the trace radius
          (LocalVariables|SetWeaponTraceDistanceIncrements (/ 1.0 (Math|Conversions|ToFloat(Integer) (Math|Float|Round (/ (LocalVariables|GetWeaponDistanceTravelled) (Utilities|Struct|BreakF_PropDestruction_Weapon_NotifyData (Variables|WeaponTrace|GetLatestWeaponNotifyData)))))))
          (for _index (range 1 (Math|Float|Round (/ (LocalVariables|GetWeaponDistanceTravelled) (Utilities|Struct|BreakF_PropDestruction_Weapon_NotifyData (Variables|WeaponTrace|GetLatestWeaponNotifyData)))))
            (Utilities|Array|Add (LocalVariables|GetNewTracePoints) (Utilities|Struct|MakeF_PropDestruction_WeaponTracePoints (Math|Vector|Lerp(Vector) _tracestart_4 (Variables|WeaponTrace|GetLastWeaponStartLocation) (* _index (LocalVariables|GetWeaponTraceDistanceIncrements))) (Math|Vector|Lerp(Vector) _traceend_4 (Variables|WeaponTrace|GetLastWeaponEndLocation) (* _index (LocalVariables|GetWeaponTraceDistanceIncrements))))))
          (else
            ;;[0.8281 0 1] If no gaps in trace, only run trace once
            (Utilities|Array|Add (LocalVariables|GetNewTracePoints) (Utilities|Struct|MakeF_PropDestruction_WeaponTracePoints _tracestart_2 _traceend_2)))))
      (:then_3
        (Utilities|DebugLevelGate
          (:Minimal
            _)
          (:Maximum
            ;[0 1 0.1094] Draw debug - velocity text
            (Rendering|Debug|DrawDebugString (Variables|WeaponTrace|GetLastWeaponEndLocation) (Utilities|String|ToString(Integer) (Math|Float|Truncate (WeaponVelocity|ProcessWeaponVelocity (LocalVariables|GetNewWeaponVelocity)))) 0 (Debug|GetDebugColourfromVelocity (WeaponVelocity|ProcessWeaponVelocity (LocalVariables|GetNewWeaponVelocity))) (Variables|Debug|GetDebugDrawTime))))
        ;[0 0.2031 1] Draw debug - weapon trail
        (Rendering|Debug|DrawDebugArrow (Variables|WeaponTrace|GetLastWeaponEndLocation) (.TraceEnd (Utilities|Struct|BreakF_PropDestruction_WeaponTraceData (Variables|WeaponTrace|GetLastWeaponTraceData))) 0.0 (Debug|GetDebugColourfromVelocity (WeaponVelocity|ProcessWeaponVelocity (LocalVariables|GetNewWeaponVelocity))) (Variables|Debug|GetDebugDrawTime) 1.0)
        ;[1 0 0.9375] Draw debug - increment points
        (for _array_element (LocalVariables|GetNewTracePoints)
          (Rendering|Debug|DrawDebugPoint (.TraceStart (Utilities|Struct|BreakF_PropDestruction_WeaponTracePoints _array_element)) 1e+01 "(R=0.022685,G=0.000000,B=1.000000,A=1.000000)" (Variables|Debug|GetDebugDrawTime))
          (Rendering|Debug|DrawDebugPoint (.TraceEnd (Utilities|Struct|BreakF_PropDestruction_WeaponTracePoints _array_element)) 1e+01 "(R=1.000000,G=0.000000,B=0.971273,A=1.000000)" (Variables|Debug|GetDebugDrawTime))))
      (:then_4
        ;[0.8047 0 1] Set new location to last weapon velocity location
        (Variables|WeaponTrace|SetLastWeaponEndLocation _traceend_3)
        (Variables|WeaponTrace|SetLastWeaponStartLocation _tracestart_3)
        ;[0 0.01562 1] Return new weapon swing data
        (return (LocalVariables|GetNewWeaponVelocity) (LocalVariables|GetNewWeaponVelocityNormal) (LocalVariables|GetNewTracePoints) false)))
    (else
      ;[0 0.6953 1] Set initial last normal velocity location if it has not yet been set, return failed
      (Variables|WeaponTrace|SetLastWeaponEndLocation _traceend)
      (Variables|WeaponTrace|SetLastWeaponStartLocation _tracestart)
      (return 0.0 "0, 0, 0" 0 true))))

(fn AccululateDeltVelocity
  (params (NewDeltVelocity :type Float%20%28double-precision%29))
  ;[1 0.9375 0] Add delt velocity to swing total
  (Variables|WeaponVelocity|SetLastHitTotalDeltVelocity (+ NewDeltVelocity (Variables|WeaponVelocity|GetLastHitTotalDeltVelocity)))
  (return))

(fn ForEachHitActorTags
  (params (Selection :type Name))
  (bind _weapon_velocity (Variables|WeaponVelocity|GetWeapon%20Velocity))
  (bind _processedvelocity (WeaponVelocity|ProcessWeaponVelocity _weapon_velocity))
  (switch name Selection
    (:DestructibleProp
      ;[0.2422 1 0] Prop tag logic
      (bind _ownerpropdestructioncomponentref (Variables|Default|GetOwnerPropDestructionComponentRef)
        (:then
          (Default|TriggerWeaponTraceDestruction _ownerpropdestructioncomponentref (Variables|WeaponTrace|GetTraceActorsToIgnore) (Variables|WeaponTrace|GetLastHitActorIndex) (Variables|WeaponTrace|GetLatestWeaponNotifyData) (Variables|WeaponTrace|GetLastWeaponTraceData) (Variables|WeaponTrace|GetLastValidHitResult) (Variables|WeaponVelocity|GetWeapon%20Velocity%20Normal) _processedvelocity (Variables|WeaponVelocity|GetWeaponVelocityRangeClamped))
          ;[0.4297 1 0] Add to accumulated velocity if directional destruction sphere spawn was successful
          (WeaponVelocity|AccululateDeltVelocity _processedvelocity))
        (:else)))
    (:HardSurface
      ;[1 0.4922 0] Run hard surface hit react check and logic if bDoHardSurfaceHitReact is true
      (WeaponHitReact|HardSurfaceHitReact (Variables|WeaponHardSurfaceHitReaction|GetbDoHardSurfaceHitReact)))))

(fn HardSurfaceHitReact
  (params (bDoHitReact :type Boolean))
  (if bDoHitReact
    ;[1 0.1641 0] Check if hit react angle threshold is met
    (if (WeaponHitReact|DoesHitMeetHitReactThreshold (Variables|WeaponTrace|GetLastValidHitResult) (Variables|WeaponVelocity|GetWeapon%20Velocity%20Normal) (Variables|WeaponHardSurfaceHitReaction|GetHardSurfaceReactAngleThreshold))
      ;[0 1 0.6719] Play hit react montage
      (Animation|Montage|MontagePlay (Components|SkeletalMesh|GetAnimInstance (Variables|Default|GetOwnerSkeletalMeshRef)) (Variables|WeaponHardSurfaceHitReaction|GetHardSurfaceHitReactMontage) 1.0 "MontageLength" 0.0 true))
    ;[1 0 0.4922] Spawn collision sparks
    (WeaponHitEffects|SpawnWeaponCollisionEffects (Variables|WeaponHardSurfaceHitReaction|GetWeaponCollisionSparks))
    (return)))

(fn DoesHitMeetHitReactThreshold
  (params (HitResult :type Hit%20Result%20Structure%20%28by%20ref%29) (WeaponVelocityNormal :type Vector) (HitReactThreshold :type Float%20%28double-precision%29))
  (return (< (Class|KismetMathLibrary|DegAcos (Math|Vector|DotProduct (* (.Normal (Collision|BreakHitResult HitResult)) -1.0) WeaponVelocityNormal)) HitReactThreshold)))

(fn SpawnWeaponCollisionEffects
  (params (SystemTemplate :type Niagara%20System%20Object%20Reference))
  (bind _lastvalidhitresult (Variables|WeaponTrace|GetLastValidHitResult))
  (bind _location (Collision|BreakHitResult _lastvalidhitresult))
  ;[0 0.5781 1] Spawn particle at collision location and weapon inverse velocity direction
  (bind _returnvalue (Niagara|SpawnSystematLocation SystemTemplate _location (Math|Conversions|RotationFromXVector (* (Variables|WeaponVelocity|GetWeapon%20Velocity%20Normal) -1.0))))
  (Audio|PlaySoundatLocation "/Game/PropDestructionSystem/DestructablePropsSamples/SampleProps_Effects/Sparks/SC_PropDestruction_Sword_Hit.SC_PropDestruction_Sword_Hit" _location "0, 0, 0" 1.0 1.0 0.0 0 0 0 0)
  (return _returnvalue))